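; BP_Ball is a physics-driven ball that moves at a constant speed and reports its destruction to BP_VRGameMode.
; Launch gives the mesh a velocity-change impulse along its forward vector.
; Every tick, ClampVelocity clamps the velocity magnitude to Speed as both minimum and maximum, so direction comes from physics while speed stays fixed.
; On BeginPlay it caches the game mode, then calls OnBallDestroyed on it when destroyed.
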(event `self.ReceiveDestroyed`
  (`/Game/Blueprints/BP_VRGameMode.On Ball Destroyed` (`self.Game Mode`)))

(event `self.ReceiveBeginPlay`
  (bind _asbp_vrgame_mode (cast `/Game/Blueprints/BP_VRGameMode` (`GameplayStatics.GetGameMode`)))
  (set `self.Game Mode` _asbp_vrgame_mode))

(event `self.ReceiveTick`
  (params (DeltaSeconds :type "Float (single-precision)"))
  (`self.Clamp Velocity`))

(event `Launch`
  (bind _ballmesh (`self.BallMesh`))
  (`PrimitiveComponent.AddImpulse` _ballmesh (`SceneComponent.GetForwardVector` _ballmesh) "None" true))

(event `Clamp Velocity`
  (bind _speed (`self.Speed`))
  (`PrimitiveComponent.SetPhysicsLinearVelocity` (`self.BallMesh`) (`KismetMathLibrary.ClampVectorSize` (`self.GetVelocity`) _speed _speed) false "None"))

(fn `UserConstructionScript`)