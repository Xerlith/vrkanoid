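; BP_Block is a destructible block for a VR game, with a score value and hit points shown on an HP widget.
; The construction script picks a random BlockTypes data table row to set color, score and hit points.
; Each hit decrements hit points, updates the widget and destroys the actor at zero or below.
; Both BeginPlay and Destroyed call DeregisterBlock on the VR game mode.
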(event `self.ReceiveBeginPlay`
  (bind _aswbp_block_hp (cast `/Game/UI/WBP_BlockHP` (`WidgetComponent.GetUserWidgetObject` (`self.HP Display`))))
  (set `/Game/UI/WBP_BlockHP.HP` (`self.Hit Points`) _aswbp_block_hp)
  (bind _asbp_vrgame_mode (cast `/Game/Blueprints/BP_VRGameMode` (`GameplayStatics.GetGameMode`)))
  (`/Game/Blueprints/BP_VRGameMode.Deregister Block` _asbp_vrgame_mode (`|ConvertAsset` self)))

(event `self.ReceiveDestroyed`
  (bind _asbp_vrgame_mode (cast `/Game/Blueprints/BP_VRGameMode` (`GameplayStatics.GetGameMode`)))
  (`/Game/Blueprints/BP_VRGameMode.Deregister Block` _asbp_vrgame_mode (`|ConvertAsset` self)))

(event `self.HandleBeingHit`
  (bind _result (`/Engine/EditorBlueprintResources/StandardMacros.DecrementInt` (`self.Hit Points`))
    (:`  `
      (bind _output_get (set `self.Hit Points` _result))
      (bind _aswbp_block_hp (cast `/Game/UI/WBP_BlockHP` (`WidgetComponent.GetUserWidgetObject` (`self.HP Display`))))
      (bind _output_get_2 (set `/Game/UI/WBP_BlockHP.HP` _output_get _aswbp_block_hp))
      (`/Engine/EditorBlueprintResources/StandardMacros.CompareInt` _output_get_2
        (:`==`
          _)
        (:`<`
          _))
      (`self.K2_DestroyActor`))))

(fn `UserConstructionScript`
  (locals (Material :type "MaterialInstanceDynamic Object Reference"))
  (bind _outrownames (`DataTableFunctionLibrary.GetDataTableRowNames` "/Game/DataStructures/BlockTypes.BlockTypes"))
  (bind _returnvalue (`|GetDataTableRow` "/Game/DataStructures/BlockTypes.BlockTypes" (`|GetArrayItem` _outrownames (`KismetMathLibrary.RandomInteger` (`KismetArrayLibrary.Array_Length` _outrownames))))
    (:`then`
      (bind _returnvalue_2 (`PrimitiveComponent.CreateDynamicMaterialInstance` (`self.Cube`) 0 "/Engine/EngineDebugMaterials/M_SimpleOpaque.M_SimpleOpaque" "None"))
      (`MaterialInstanceDynamic.SetVectorParameterValue` _returnvalue_2 "Color" (`KismetMathLibrary.Conv_ColorToLinearColor` (break `/Game/DataStructures/BlockType` _returnvalue)))
      (set `self.Score` (`.Score_10_39DFCB5D439D24825D3E359E38E228F6` (break `/Game/DataStructures/BlockType` _returnvalue)))
      (set `self.Hit Points` (`.HitPoints_6_8840A5F047BE1509C0D10796CC49B96E` (break `/Game/DataStructures/BlockType` _returnvalue))))))