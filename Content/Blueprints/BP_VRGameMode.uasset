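; VR game mode for a ball-and-block game that tracks score, remaining balls and game state.
; Blocks register themselves through events, and deregistering one adds its score to the total.
; Starting or resetting reloads the "Boxes" streamed level and restores balls and score; starting also spawns a ball through the SM_PlayerPlatform actor.
; Each destroyed ball decrements the count, then either respawns a ball or switches to the game-over state.
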(event `self.ReceiveBeginPlay`
  (`self.Reset Game`)
  (set `self.E_GameState` "NewEnumerator2"))

(event `Deregister Block`
  (params (Block :type "/Game/Blueprints/BP_Block Soft Object Reference (by ref)"))
  (bind _output (`|ConvertAsset` Block))
  (`KismetArrayLibrary.Array_RemoveItem` (`self.Existing Blocks`) _output)
  (`self.Increment Score` (`/Game/Blueprints/BP_Block.Score` _output)))

(event `Register Block`
  (params (Block :type "/Game/Blueprints/BP_Block Soft Object Reference (by ref)"))
  (`KismetArrayLibrary.Array_Add` (`self.Existing Blocks`) (`|ConvertAsset` Block)))

(event `Increment Score`
  (params (Points :type Integer))
  (set `self.Current Score` (+ Points (`self.Current Score`))))

(event `Reset Game`
  (`self.Reload blocks`)
  (set `self.Current Balls` (`self.Max Balls`))
  (set `self.Current Score` 0))

(event `On Ball Destroyed`
  (bind _result (`/Engine/EditorBlueprintResources/StandardMacros.DecrementInt` (`self.Current Balls`))
    (:`  `
      (`/Engine/EditorBlueprintResources/StandardMacros.CompareInt` _result
        (:`>`
          (`self.Spawn Ball`))
        (:`==`
          (`self.Game Over` :!label _label))
        (:`<`
          (goto _label))))))

(event `Game Over`
  (set `self.E_GameState` "NewEnumerator1"))

(event `Start Game`
  (`self.Reset Game`)
  (set `self.E_GameState` "NewEnumerator0")
  (`self.Spawn Ball`))

(event `Reload blocks`
  (`GameplayStatics.UnloadStreamLevel` "Boxes")
  (`GameplayStatics.LoadStreamLevel` "Boxes" true))

(event `Spawn Ball`
  (bind _returnvalue (`GameplayStatics.GetActorOfClass` "/Game/StarterContent/Architecture/SM_PlayerPlatform.SM_PlayerPlatform_C"))
  (`/Game/StarterContent/Architecture/SM_PlayerPlatform.Spawn Ball` _returnvalue))

(fn `UserConstructionScript`)